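; BP_Grump is an AI companion that follows the player or gathers wood and rock to hand over.
; Interaction options and idle or following timers switch its tasks by setting Blackboard keys.
; While searching, its detector overlap targets unused "Resource"-tagged actors, and a delayed task loop adds random yields until the resource is spent.
; It drives talk and option widgets and reports totals and autonomy changes to the player through messages.
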(event `self.ReceiveBeginPlay`
  (`|ExecutionSequence`
    (:`then_0`
      ;[1 1 1] Casting to Widget
      (bind _asw_text_box (cast `/Game/Josh/Widget/W_TextBox` (`WidgetComponent.GetUserWidgetObject` (`self.W_TalkBox`))))
      (set `self.As W Text Box` _asw_text_box)
      (bind _asw_npcinteraction (cast `/Game/Josh/Widget/W_NPCInteraction` (`WidgetComponent.GetUserWidgetObject` (`self.W_InteractionOptions`))))
      (set `self.As W NPCInteraction` _asw_npcinteraction)
      (bind _asbp_third_person_character (cast `/Game/ThirdPerson/Blueprints/BP_ThirdPersonCharacter` (`GameplayStatics.GetPlayerCharacter` 0)))
      (set `self.As BP Third Person Character` _asbp_third_person_character)
      (set `/Game/ThirdPerson/Blueprints/BP_ThirdPersonCharacter.Grump` self _asbp_third_person_character))
    (:`then_1`
      (`self.ChasePlayer`))
    (:`then_2`
      ;[1 1 1] Timer per continuouse actions
      (`KismetSystemLibrary.K2_SetTimer` null "SameText?" 4.0 true)
      (`KismetSystemLibrary.K2_SetTimer` null "IdleTooLong" 7.5 true)
      (`KismetSystemLibrary.K2_SetTimer` null "FollowingTooLong" 7.5 true))))

(event `/Game/Josh/BPI/BPI_NPC.GrumpScore`
  (message `/Game/Josh/BPI/BPI_Score.GrumpScore` (`GameplayStatics.GetPlayerCharacter` 0) (`self.TotalWoodCollected`) (`self.TotalRockCollected`)))

(event `IdleTooLong`
  ;[0 0.3355 1] Idle Too Long
  (if (`self.idle?`)
    (set `self.idle?` false)
    (message `/Game/Josh/BPI/BPI_Score.GrumpAutonomy` (`GameplayStatics.GetPlayerCharacter` 0))
    (`self.SearchResources`)))

(event `self.ReceiveTick`
  (params (DeltaSeconds :type "Float (single-precision)"))
  ;[0.7466 0 1] Testing
)

(event `FollowingTooLong`
  (if (`self.chasing?`)
    (if (and (== (`self.RockInventory`) 0) (== (`self.WoodInventory`) 0))
      (set `self.chasing?` false)
      (message `/Game/Josh/BPI/BPI_Score.GrumpAutonomy` (`GameplayStatics.GetPlayerCharacter` 0))
      (`self.SearchResources`))))

(event `SameText?`
  (bind _currentjob (`/Game/Josh/Widget/W_TextBox.CurrentJob` (`self.As W Text Box`)))
  ;[0 0.3355 1] Remove text after a while
  (if (== _currentjob (`self.TextSameLast?`))
    (set `/Game/Josh/Widget/W_TextBox.CurrentJob` 0 (`self.As W Text Box`))
    (else
      (set `self.TextSameLast?` _currentjob))))

(event `self.SelectOption`
  (params (Option :type Integer))
  ;[1 0 0] Player Interaction on AI
  (set `self.OptionSelected` Option)
  (`KismetSystemLibrary.PrintString` (`KismetStringLibrary.Conv_IntToString` Option))
  (if (== (`self.OptionSelected`) 1)
    (`self.StopCurrentTask`)
    (`self.Follow/UnFollow`)
    (elif (== (`self.OptionSelected`) 2)
      (`self.StopCurrentTask`)
      (if (`/Game/Josh/Widget/W_NPCInteraction.hasMaterials?` (`self.As W NPCInteraction`))
        (`self.GiveMaterialToPlayer`)
        (else
          (`self.SearchResources`))))))

(event `self.InteractionRange.OnComponentBeginOverlap`
  (params (OverlappedComponent :type "PrimitiveComponent Object Reference") (OtherActor :type "Actor Object Reference") (OtherComp :type "PrimitiveComponent Object Reference") (OtherBodyIndex :type Integer) (bFromSweep :type Boolean) (SweepResult :type "HitResult Structure (by ref)"))
  ;[0 0.3355 1] Widget proximity
  (if (not (`self.interactionComplete?`))
    ;;[1 1 1] Interact Text appears when Player nearby
    (if (== (`GameplayStatics.GetPlayerCharacter` 0) OtherActor)
      (`SceneComponent.SetVisibility` (`self.W_InteractionOptions`) true false)
      (if (or (> (`self.RockInventory`) 0) (> (`self.WoodInventory`) 0))
        (set `/Game/Josh/Widget/W_NPCInteraction.hasMaterials?` true (`self.As W NPCInteraction`))
        (set `/Game/Josh/Widget/W_TextBox.CurrentJob` 10 (`self.As W Text Box`))))))

(event `Follow/UnFollow`
  ;[1 0 0] Option 1
  ;;[1 1 1] Value of FollowMe in BB
  (if (`BlackboardComponent.GetValueAsBool` (`AIBlueprintHelperLibrary.GetBlackboard` null) "FollowMe")
    ;;[1 1 1] Stop Chase
    (`BlackboardComponent.SetValueAsBool` (`AIBlueprintHelperLibrary.GetBlackboard` null) "FollowMe" false)
    (set `/Game/Josh/Widget/W_NPCInteraction.isChasing?` false (`self.As W NPCInteraction`))
    (set `/Game/Josh/Widget/W_TextBox.CurrentJob` 10 (`self.As W Text Box`))
    (set `self.idle?` true)
    (else
      ;;[1 1 1] Start Chase
      (`BlackboardComponent.SetValueAsBool` (`AIBlueprintHelperLibrary.GetBlackboard` null) "FollowMe" true :!label _label)
      (set `/Game/Josh/Widget/W_NPCInteraction.isChasing?` true (`self.As W NPCInteraction`))
      (set `/Game/Josh/Widget/W_TextBox.CurrentJob` 10 (`self.As W Text Box`))
      (set `self.chasing?` true))))

(event `self.ResourceDetector.OnComponentBeginOverlap`
  (params (OverlappedComponent :type "PrimitiveComponent Object Reference") (OtherActor :type "Actor Object Reference") (OtherComp :type "PrimitiveComponent Object Reference") (OtherBodyIndex :type Integer) (bFromSweep :type Boolean) (SweepResult :type "HitResult Structure (by ref)"))
  (bind _returnvalue_location (`KismetMathLibrary.BreakTransform` (`self.GetTransform` (`self.resourceTarget`))))
  ;[0.005213 1 0] Check for Resources
  (if (`self.searchingResources`)
    (if (`KismetArrayLibrary.Array_Contains` (`self.allResorces`) OtherActor)
      (if (not (`self.ActorHasTag` OtherActor "Used"))
        (set `self.resourceTarget` OtherActor)
        (`KismetSystemLibrary.PrintString` (`KismetSystemLibrary.GetDisplayName` (`self.resourceTarget`)))
        (`BlackboardComponent.SetValueAsVector` (`AIBlueprintHelperLibrary.GetBlackboard` null) "TargetLocation" _returnvalue_location)
        (`BlackboardComponent.SetValueAsBool` (`AIBlueprintHelperLibrary.GetBlackboard` null) "resourceFound?" true)
        (`BlackboardComponent.SetValueAsObject` (`AIBlueprintHelperLibrary.GetBlackboard` null) "TargetResource" (`self.resourceTarget`))))))

(event `self.InteractionRange.OnComponentEndOverlap`
  (params (OverlappedComponent :type "PrimitiveComponent Object Reference") (OtherActor :type "Actor Object Reference") (OtherComp :type "PrimitiveComponent Object Reference") (OtherBodyIndex :type Integer))
  ;[0 0.3355 1] Widget proximity
  (if (not (`self.interactionComplete?`))
    ;;[1 1 1] Interact Text appears when Player nearby
    (if (== (`GameplayStatics.GetPlayerCharacter` 0) OtherActor)
      (`SceneComponent.SetVisibility` (`self.W_InteractionOptions`) false false))))

(event `ChasePlayer`
  ;[1 0 0] Option 1
  (goto _label))

(event `TaskTimeCompleted`
  ;[0.005213 1 0] Interacting with resource
  ;;[1 1 1] Check Resource Integrity
  (bind _result (`/Engine/EditorBlueprintResources/StandardMacros.IncrementInt` (`self.ResourceSuccesses`))
    (:`  `
      (`KismetSystemLibrary.PrintString` (`KismetStringLibrary.Concat_StrStr` "Resource Successes: " (`KismetTextLibrary.Conv_TextToString` (`KismetTextLibrary.Conv_IntToText` _result))))
      (if (>= _result 4)
        ;;[1 1 1] Uses up the Resource
        (message `/Game/Josh/BPI/BPI_Interact.InteractionCompleted` (`self.resourceTarget`))
        (`self.CompletedGatheringResource`)
        (else
          ;;[1 1 1] Gain Resource and Loops to the beginning
          (`self.Gain Resource`)
          (`self.DoingTask`))))))

(event `StopCurrentTask`
  ;[1 0 0] Stop Current Task
  (if (== (`self.OptionSelected`) 1)
    ;;[1 1 1] DeSelect 2
    (`BlackboardComponent.SetValueAsBool` (`AIBlueprintHelperLibrary.GetBlackboard` null) "gatherResources" false)
    (`SceneComponent.SetVisibility` (`self.ResourceDetector`) false false)
    (set `self.searchingResources` false)
    (elif (== (`self.OptionSelected`) 2)
      ;;[1 1 1] DeSelect 1
      (`BlackboardComponent.SetValueAsBool` (`AIBlueprintHelperLibrary.GetBlackboard` null) "FollowMe" false)
      (set `/Game/Josh/Widget/W_NPCInteraction.isChasing?` false (`self.As W NPCInteraction`))
      (set `/Game/Josh/Widget/W_TextBox.CurrentJob` 10 (`self.As W Text Box`)))))

(event `GiveMaterialToPlayer`
  (bind _returnvalue (`GameplayStatics.GetPlayerCharacter` 0))
  (bind _as_bp_third_person_character (`self.As BP Third Person Character`))
  (bind _as_bp_third_person_character_2 (`self.As BP Third Person Character`))
  ;[1 0 0] Option 2a
  (message `/Game/Josh/BPI/BPI_MiniGames.TreeMiniGameIncrease` _returnvalue (`self.WoodInventory`))
  (message `/Game/Josh/BPI/BPI_MiniGames.RockMiniGameIncrease` _returnvalue (`self.RockInventory`))
  ;;[1 1 1] To check which player has collected VS AI
  (set `/Game/ThirdPerson/Blueprints/BP_ThirdPersonCharacter.TreesICollected` (- (`/Game/ThirdPerson/Blueprints/BP_ThirdPersonCharacter.TreesICollected` _as_bp_third_person_character_2) (`self.WoodInventory`)) _as_bp_third_person_character_2)
  (set `/Game/ThirdPerson/Blueprints/BP_ThirdPersonCharacter.RockICollected` (- (`/Game/ThirdPerson/Blueprints/BP_ThirdPersonCharacter.RockICollected` _as_bp_third_person_character) (`self.RockInventory`)) _as_bp_third_person_character)
  (set `self.WoodInventory` 0)
  (set `self.RockInventory` 0)
  (set `/Game/Josh/Widget/W_NPCInteraction.hasMaterials?` false (`self.As W NPCInteraction`))
  (set `/Game/Josh/Widget/W_TextBox.CurrentJob` 10 (`self.As W Text Box`))
  (set `self.idle?` true))

(event `Gain Resource`
  ;[0.005213 1 0] Interacting with resource
  ;;[1 1 1] Gain resource with Target
  (`/Engine/EditorBlueprintResources/StandardMacros.IsValid` (`self.resourceTarget`)
    (:`Is Valid`
      (if (`self.ActorHasTag` (`self.resourceTarget`) "Tree")
        (bind _output_get (set `self.WoodInventory` (+ (`self.WoodInventory`) (`KismetMathLibrary.RandomIntegerInRange` 0 3))))
        (set `self.TotalWoodCollected` (+ _output_get (`self.TotalWoodCollected`)))
        (set `/Game/Josh/Widget/W_TextBox.CurrentJob` 10 (`self.As W Text Box`))
        (elif (`self.ActorHasTag` (`self.resourceTarget`) "Rock")
          (bind _output_get_2 (set `self.RockInventory` (+ (`self.RockInventory`) (`KismetMathLibrary.RandomIntegerInRange` 0 3))))
          (set `self.TotalRockCollected` (+ _output_get_2 (`self.TotalRockCollected`)))
          (set `/Game/Josh/Widget/W_TextBox.CurrentJob` 10 (`self.As W Text Box`)))))))

(event `SearchResources`
  ;[1 0 0] Option 2b
  (`self.ClearResourcesList`)
  (bind _outactors (`GameplayStatics.GetAllActorsWithTag` "Resource"))
  (set `self.allResorces` _outactors)
  (`BlackboardComponent.SetValueAsBool` (`AIBlueprintHelperLibrary.GetBlackboard` null) "gatherResources" true)
  (set `self.searchingResources` true)
  (set `/Game/Josh/Widget/W_TextBox.CurrentJob` 10 (`self.As W Text Box`)))

(event `ClearResourcesList`
  ;[1 1 1] Resource Clear
  (`KismetArrayLibrary.Array_Clear` (`self.allResorces`))
  (`BlackboardComponent.SetValueAsBool` (`AIBlueprintHelperLibrary.GetBlackboard` null) "resourceFound?" false))

(event `self.MatchSpeed`
  (params (`chasingPlayer?` :type Boolean))
  (bind _charactermovement (`self.CharacterMovement`))
  ;[0.101 0.101 0.101] Not being used
  ;;[1 1 1] UnUsed
  (if `chasingPlayer?`
    (set `CharacterMovementComponent.MaxWalkSpeed` 450.0 _charactermovement)
    (else
      (set `CharacterMovementComponent.MaxWalkSpeed` 350.0 _charactermovement))))

(event `CompletedGatheringResource`
  ;[0.005213 1 0] Interacting with resource
  ;;[1 1 1] Completed Resources Gathering
  (`KismetSystemLibrary.PrintText` "DONEMYJOB")
  (set `self.resourceTarget` null)
  (set `self.ResourceSuccesses` 0)
  (`BlackboardComponent.SetValueAsBool` (`AIBlueprintHelperLibrary.GetBlackboard` null) "doingResources" false)
  (`self.SelectOption` 1))

(event `self.DoingTask`
  ;[0.005213 1 0] Doing Task
  (`BlackboardComponent.SetValueAsBool` (`AIBlueprintHelperLibrary.GetBlackboard` null) "doingResources" true)
  (`KismetSystemLibrary.Delay` (`KismetMathLibrary.RandomFloatInRange` 1.0 2.0))
  (`self.TaskTimeCompleted`))

(fn `UserConstructionScript`)