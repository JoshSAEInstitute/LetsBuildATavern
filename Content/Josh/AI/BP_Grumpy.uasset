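; BP_Grumpy is an AI NPC that the player can order to follow or to gather resources.
; An interaction widget shows while the player is in range, and SelectOption cancels the other task, then toggles following or starts a search.
; Both orders drive Blackboard keys.
; While searching, the ResourceDetector overlap checks actors against the cached "Resource"-tagged list, skips "Used" ones and writes the target location to the Blackboard.
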(event `self.ResourceDetector.OnComponentBeginOverlap`
  (params (OverlappedComponent :type "PrimitiveComponent Object Reference") (OtherActor :type "Actor Object Reference") (OtherComp :type "PrimitiveComponent Object Reference") (OtherBodyIndex :type Integer) (bFromSweep :type Boolean) (SweepResult :type "HitResult Structure (by ref)"))
  (bind _returnvalue (`AIBlueprintHelperLibrary.GetBlackboard` null))
  (bind _resourcetarget (`self.resourceTarget`))
  (bind _returnvalue_location (`KismetMathLibrary.BreakTransform` (`self.GetTransform` (`self.resourceTarget`))))
  ;[1 1 1] Check for Resources
  (set `self.resourceTarget` OtherActor)
  (if (`self.searchingResources`)
    (if (`KismetArrayLibrary.Array_Contains` (`self.allResorces`) _resourcetarget)
      (if (not (`self.ActorHasTag` _resourcetarget "Used"))
        (`BlackboardComponent.SetValueAsVector` _returnvalue "TargetLocation" _returnvalue_location)
        (`BlackboardComponent.SetValueAsBool` _returnvalue "resourceFound?" true)))))

(event `self.InteractionRange.OnComponentBeginOverlap`
  (params (OverlappedComponent :type "PrimitiveComponent Object Reference") (OtherActor :type "Actor Object Reference") (OtherComp :type "PrimitiveComponent Object Reference") (OtherBodyIndex :type Integer) (bFromSweep :type Boolean) (SweepResult :type "HitResult Structure (by ref)"))
  (if (not (`self.interactionComplete?`))
    ;[1 1 1] Interact Text appears when Player nearby
    (if (== (`GameplayStatics.GetPlayerCharacter` 0) OtherActor)
      (`SceneComponent.SetVisibility` (`self.W_InteractionOptions`) true false))))

(event `self.InteractionRange.OnComponentEndOverlap`
  (params (OverlappedComponent :type "PrimitiveComponent Object Reference") (OtherActor :type "Actor Object Reference") (OtherComp :type "PrimitiveComponent Object Reference") (OtherBodyIndex :type Integer))
  (if (not (`self.interactionComplete?`))
    ;[1 1 1] Interact Text appears when Player nearby
    (if (== (`GameplayStatics.GetPlayerCharacter` 0) OtherActor)
      (`SceneComponent.SetVisibility` (`self.W_InteractionOptions`) false false))))

(event `StopCurrentTask`
  (if (== (`self.OptionSelected`) 1)
    ;[1 1 1] DeSelect 2
    (`BlackboardComponent.SetValueAsBool` (`AIBlueprintHelperLibrary.GetBlackboard` null) "gatherResources" false)
    (`SceneComponent.SetVisibility` (`self.ResourceDetector`) false false)
    (set `self.searchingResources` false)
    (elif (== (`self.OptionSelected`) 2)
      ;[1 1 1] DeSelect 1
      (`BlackboardComponent.SetValueAsBool` (`AIBlueprintHelperLibrary.GetBlackboard` null) "FollowMe" false)
      (set `/Game/Josh/Widget/W_NPCInteraction.isChasing?` false (`self.As W NPCInteraction`)))))

(event `/Game/Josh/BPI/BPI_NPC.MatchSpeed`
  (params (`chasingPlayer?` :type Boolean))
  (bind _charactermovement (`self.CharacterMovement`))
  ;[1 1 1] UnUsed
  (if `chasingPlayer?`
    (set `CharacterMovementComponent.MaxWalkSpeed` 450.0 _charactermovement)
    (else
      (set `CharacterMovementComponent.MaxWalkSpeed` 350.0 _charactermovement))))

(event `/Game/Josh/BPI/BPI_Interact.SelectOption`
  (params (Option :type Integer))
  (set `self.OptionSelected` Option)
  (`KismetSystemLibrary.PrintString` (`KismetStringLibrary.Conv_IntToString` Option))
  ;[1 1 1] Casting to Widget
  (bind _asw_npcinteraction (cast `/Game/Josh/Widget/W_NPCInteraction` (`WidgetComponent.GetUserWidgetObject` (`self.W_InteractionOptions`))))
  (set `self.As W NPCInteraction` _asw_npcinteraction)
  (if (== (`self.OptionSelected`) 1)
    (`self.StopCurrentTask`)
    ;[1 1 1] Option 1
    ;;[1 1 1] Value of FollowMe in BB
    (if (`BlackboardComponent.GetValueAsBool` (`AIBlueprintHelperLibrary.GetBlackboard` null) "FollowMe")
      ;;[1 1 1] Stop Chase
      (`BlackboardComponent.SetValueAsBool` (`AIBlueprintHelperLibrary.GetBlackboard` null) "FollowMe" false)
      (set `/Game/Josh/Widget/W_NPCInteraction.isChasing?` false (`self.As W NPCInteraction`))
      (else
        ;;[1 1 1] Start Chase
        (`BlackboardComponent.SetValueAsBool` (`AIBlueprintHelperLibrary.GetBlackboard` null) "FollowMe" true)
        (set `/Game/Josh/Widget/W_NPCInteraction.isChasing?` true (`self.As W NPCInteraction`))))
    (elif (== (`self.OptionSelected`) 2)
      (`self.StopCurrentTask`)
      ;[1 1 1] Option 2
      (`self.ClearResourcesList`)
      (bind _outactors (`GameplayStatics.GetAllActorsWithTag` "Resource"))
      (set `self.allResorces` _outactors)
      (`BlackboardComponent.SetValueAsBool` (`AIBlueprintHelperLibrary.GetBlackboard` null) "gatherResources" true)
      (set `self.searchingResources` true))))

(event `ClearResourcesList`
  (`KismetArrayLibrary.Array_Clear` (`self.allResorces`))
  (`BlackboardComponent.SetValueAsBool` (`AIBlueprintHelperLibrary.GetBlackboard` null) "resourceFound?" false))

(fn `UserConstructionScript`)