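; BP_Rock is an interactable rock that starts the player's rock minigame and respawns after use.
; It picks a random mesh at BeginPlay, and a sphere overlap toggles an interact prompt for the player.
; Interact calls RockMiniGameMessage on the player character.
; Completion swaps to a used mesh, adds a "Used" tag, and starts a short timer that re-randomises the mesh and re-enables interaction.
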(event `self.ReceiveBeginPlay`
  ;[1 1 1] Set Random Tree Mesh
  (`StaticMeshComponent.SetStaticMesh` (`self.Rock`) (`KismetArrayLibrary.Array_Random` (`self.RockList`)) :!label _label))

(event `SetMesh`
  ;[1 1 1] Set Random Tree Mesh
  (goto _label))

(event `self.Sphere.OnComponentBeginOverlap`
  (params (OverlappedComponent :type "PrimitiveComponent Object Reference") (OtherActor :type "Actor Object Reference") (OtherComp :type "PrimitiveComponent Object Reference") (OtherBodyIndex :type Integer) (bFromSweep :type Boolean) (SweepResult :type "HitResult Structure (by ref)"))
  ;[0 0.3355 1] Widgets
  (if (not (`self.interactionComplete?`))
    ;;[1 1 1] Interact Text appears when Player nearby
    (if (== OtherActor (`GameplayStatics.GetPlayerCharacter` 0))
      (`SceneComponent.SetVisibility` (`self.W_Interact`) true false))))

(event `self.Sphere.OnComponentEndOverlap`
  (params (OverlappedComponent :type "PrimitiveComponent Object Reference") (OtherActor :type "Actor Object Reference") (OtherComp :type "PrimitiveComponent Object Reference") (OtherBodyIndex :type Integer))
  ;[0 0.3355 1] Widgets
  (if (not (`self.interactionComplete?`))
    ;;[1 1 1] Interact Text appears when Player nearby
    (if (== (`GameplayStatics.GetPlayerCharacter` 0) OtherActor)
      (`SceneComponent.SetVisibility` (`self.W_Interact`) false false))))

(event `/Game/Josh/BPI/BPI_Interact.Interact`
  ;[0 0.3355 1] Widgets
  (`SceneComponent.SetVisibility` (`self.W_Interact`) false false)
  (message `/Game/Josh/BPI/BPI_MiniGames.RockMiniGame` (`GameplayStatics.GetPlayerCharacter` 0)))

(event `/Game/Josh/BPI/BPI_Interact.InteractionCompleted`
  (`StaticMeshComponent.SetStaticMesh` (`self.Rock`) "/Game/Kobo_ForestVillage/Meshes/SM-Rock-02.SM-Rock-02")
  (set `self.interactionComplete?` true)
  (`KismetArrayLibrary.Array_Add` (`self.Tags`) "Used")
  (`self.TimerCD`))

(event `TimerCD`
  (bind _returnvalue (`KismetSystemLibrary.K2_SetTimerDelegate` (delegate `RestartBP`) 2.0))
  (set `self.ReGrowthTimer` _returnvalue))

(event `RestartBP`
  (`KismetSystemLibrary.K2_InvalidateTimerHandle` (`self.ReGrowthTimer`))
  (`self.SetMesh`)
  (`KismetArrayLibrary.Array_RemoveItem` (`self.Tags`) "Used")
  (set `self.interactionComplete?` false))

(fn `UserConstructionScript`)