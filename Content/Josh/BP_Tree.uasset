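; BP_Tree is an interactable tree actor that shows a prompt widget when the player is nearby.
; On BeginPlay it assigns the SMTree01 mesh to its Tree component.
; Sphere overlap events toggle the Widget component's visibility for player character 0 only.
; The Interact event is a placeholder that prints a debug string.
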(event `self.ReceiveBeginPlay`
  (`StaticMeshComponent.SetStaticMesh` (`self.Tree`) "/Game/Kobo_ForestVillage/Meshes/SM-Tree-01.SM-Tree-01"))

(event `self.Sphere.OnComponentBeginOverlap`
  (params (OverlappedComponent :type "PrimitiveComponent Object Reference") (OtherActor :type "Actor Object Reference") (OtherComp :type "PrimitiveComponent Object Reference") (OtherBodyIndex :type Integer) (bFromSweep :type Boolean) (SweepResult :type "HitResult Structure (by ref)"))
  (if (== OtherActor (`GameplayStatics.GetPlayerCharacter` 0))
    (`SceneComponent.SetVisibility` (`self.Widget`) true false)))

(event `self.Sphere.OnComponentEndOverlap`
  (params (OverlappedComponent :type "PrimitiveComponent Object Reference") (OtherActor :type "Actor Object Reference") (OtherComp :type "PrimitiveComponent Object Reference") (OtherBodyIndex :type Integer))
  (if (== (`GameplayStatics.GetPlayerCharacter` 0) OtherActor)
    (`SceneComponent.SetVisibility` (`self.Widget`) false false)))

(event `/Game/Josh/BPI/BPI_Interact.Interact`
  (`KismetSystemLibrary.PrintString` "Hello"))

(fn `UserConstructionScript`)