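; Tavern actor that serves as an interactable objective, showing its objective widget while the player is inside the PlayerDetection volume.
; BeginPlay caches the player character and the W_Tavern instance from the WObjective widget component.
; Interact checks that widget's CanComplete flag, then calls GameTimerMessage on the player, switches input to game and UI with a visible cursor, and pauses the game.
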(event `self.ReceiveBeginPlay`
  (bind _asbp_third_person_character (cast `/Game/ThirdPerson/Blueprints/BP_ThirdPersonCharacter` (`GameplayStatics.GetPlayerCharacter` 0)))
  (set `self.As BP Third Person Character` _asbp_third_person_character)
  (bind _asw_tavern (cast `/Game/Josh/Widget/W_Tavern` (`WidgetComponent.GetUserWidgetObject` (`self.W_Objective`))))
  (set `self.As W Tavern` _asw_tavern))

(event `self.Player Detection.OnComponentBeginOverlap`
  (params (OverlappedComponent :type "PrimitiveComponent Object Reference") (OtherActor :type "Actor Object Reference") (OtherComp :type "PrimitiveComponent Object Reference") (OtherBodyIndex :type Integer) (bFromSweep :type Boolean) (SweepResult :type "HitResult Structure (by ref)"))
  (if (== OtherActor (`GameplayStatics.GetPlayerCharacter` 0))
    (`SceneComponent.SetVisibility` (`self.W_Objective`) true false)))

(event `self.Player Detection.OnComponentEndOverlap`
  (params (OverlappedComponent :type "PrimitiveComponent Object Reference") (OtherActor :type "Actor Object Reference") (OtherComp :type "PrimitiveComponent Object Reference") (OtherBodyIndex :type Integer))
  (if (== OtherActor (`GameplayStatics.GetPlayerCharacter` 0))
    (`SceneComponent.SetVisibility` (`self.W_Objective`) false false)))

(event `/Game/Josh/BPI/BPI_Interact.Interact`
  (if (`/Game/Josh/Widget/W_Tavern.CanComplete` (`self.As W Tavern`))
    (message `/Game/Josh/BPI/BPI_Score.Game Timer` (`GameplayStatics.GetPlayerCharacter` 0))
    (`WidgetBlueprintLibrary.SetInputMode_GameAndUIEx` (`GameplayStatics.GetPlayerController` 0) null)
    (set `PlayerController.bShowMouseCursor` true (`GameplayStatics.GetPlayerController` 0))
    (`GameplayStatics.SetGamePaused` true)))

(fn `UserConstructionScript`)